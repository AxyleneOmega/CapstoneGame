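; BP_Item is a world item pickup actor driven by an Item data asset and a Quantity.
; Its construction script applies the asset's mesh, scale and optional material override, and prints the item name.
; Interactwith adds the quantity to the player's InventorySystem, keeps any remainder, and destroys the actor once everything is successfully added.
; LookAt returns the item data, while Consumption and NewFunction are empty.
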(event EventBeginPlay)

(event Collision|EventActorBeginOverlap
  (params (OtherActor :type Actor%20Object%20Reference)))

(event EventTick
  (params (DeltaSeconds :type Float%20%28single-precision%29)))

(event EventInteractwith
  (params (PlayerCharacter :type BP%20CG%20Char%20Object%20Reference))
  (bind _inventorysystem (Variables|/Game/Capstone/Systems/Player/BP_CG_Char.BP_CG_Char_C|GetInventorySystem PlayerCharacter))
  (Utilities|IsValid _inventorysystem
    (:Is%20Valid
      (bind (_success _quantityremaining) (Default|AddtoInventory _inventorysystem (Variables|Default|GetItem) (Variables|Default|GetQuantity)))
      (bind _output_get (Variables|Default|SetQuantity _quantityremaining))
      (if (and _success (== _output_get 0))
        (Actor|DestroyActor)))))

(event EventConsumption
  (params (PlayerCharacter :type BP%20CG%20Char%20Object%20Reference)))

(event EventNewFunction)

(fn ConstructionScript
  (bind _item (Variables|Default|GetItem)
    (:then
      (Development|PrintString (Utilities|String|ToString(Text) (Variables|/Game/Capstone/Systems/Inventory/ItemDataAsset/DA_Item.DA_Item_C|GetName _item)))
      (Components|StaticMesh|SetStaticMesh (Variables|Default|GetStaticMesh) (Variables|/Game/Capstone/Systems/Inventory/ItemDataAsset/DA_Item.DA_Item_C|GetItemMesh _item))
      (Transformation|SetActorScale3D (Variables|/Game/Capstone/Systems/Inventory/ItemDataAsset/DA_Item.DA_Item_C|GetMeshScale _item))
      (bind _meshmaterialoverride (Variables|/Game/Capstone/Systems/Inventory/ItemDataAsset/DA_Item.DA_Item_C|GetMeshMaterialOverride _item)
        (:then
          (Rendering|Material|SetMaterial (Variables|Default|GetStaticMesh) 0 _meshmaterialoverride))
        (:else)))
    (:else)))

(fn Lookat
  (return (Variables|Default|GetItem)))