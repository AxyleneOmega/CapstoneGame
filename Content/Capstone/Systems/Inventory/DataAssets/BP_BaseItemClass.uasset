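; BP_BaseItemClass is a base pickable item actor driven by an Item data asset.
; Its construction script prints the item's name and applies the asset's mesh.
; Interactwith passes Item and Quantity to the player's InventorySystem, then destroys the actor without acting on the success result.
; LookAt creates a W_LookAtPickableItem widget for the item, adds it to the viewport and returns it.
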(event EventBeginPlay)

(event Collision|EventActorBeginOverlap
  (params (OtherActor :type Actor%20Object%20Reference)))

(event EventTick
  (params (DeltaSeconds :type Float%20%28single-precision%29)))

(event EventInteractwith
  (params (PlayerCharacter :type BP%20CG%20Char%20Object%20Reference))
  (bind _inventorysystem (Variables|/Game/Capstone/BP_CG_Char.BP_CG_Char_C|GetInventorySystem PlayerCharacter))
  (Utilities|IsValid _inventorysystem
    (:Is%20Valid
      (bind _success (Default|AddtoInventory _inventorysystem (Variables|Default|GetItem) (Variables|Default|GetQuantity)))
      (if _success
        _
        (else
          _))
      (Actor|DestroyActor))))

(fn ConstructionScript
  (bind _item (Variables|Default|GetItem)
    (:then
      (Development|PrintString (Utilities|String|ToString(Text) (Variables|/Game/Capstone/Systems/Inventory/DataAssets/BaseDataAssetItem.BaseDataAssetItem_C|GetName _item)))
      (Variables|Default|SetStaticMesh (Variables|/Game/Capstone/Systems/Inventory/DataAssets/BaseDataAssetItem.BaseDataAssetItem_C|GetItemMesh _item)))
    (:else)))

(fn Lookat
  (bind _returnvalue (UserInterface|CreateWidget "/Game/Capstone/Systems/Inventory/Widgets/W_LookAtPickableItem.W_LookAtPickableItem_C" 0 (Variables|Default|GetItem)))
  (UserInterface|Viewport|AddtoViewport _returnvalue 0)
  (return _returnvalue))