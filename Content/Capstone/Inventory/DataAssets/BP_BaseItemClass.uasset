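; Base actor for pickable inventory items, with its mesh and look-at prompt driven by an Item reference.
; The construction script takes the static mesh from a valid Item and prints the item's name.
; LookAt creates a W_LookAtPickableItem widget for that Item, adds it to the viewport and returns it to the caller.
; The event graph holds no active logic.
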(event EventBeginPlay)

(event Collision|EventActorBeginOverlap
  (params (OtherActor :type Actor%20Object%20Reference)))

(event EventTick
  (params (DeltaSeconds :type Float%20%28single-precision%29)))

(fn ConstructionScript
  (bind _item (Variables|Default|GetItem)
    (:then
      (Development|PrintString (Utilities|String|ToString(Text) (Variables|/Game/Capstone/Inventory/DataAssets/BaseDataAssetItem.BaseDataAssetItem_C|GetName _item)))
      (Variables|Default|SetStaticMesh (Variables|/Game/Capstone/Inventory/DataAssets/BaseDataAssetItem.BaseDataAssetItem_C|GetItemMesh _item)))
    (:else)))

(fn Lookat
  (bind _item (Variables|Default|GetItem)
    (:then
      (bind _returnvalue (UserInterface|CreateWidget "/Game/Capstone/Inventory/Widgets/W_LookAtPickableItem.W_LookAtPickableItem_C" 0 _item))
      (UserInterface|Viewport|AddtoViewport _returnvalue 0)
      (return _returnvalue))
    (:else)))