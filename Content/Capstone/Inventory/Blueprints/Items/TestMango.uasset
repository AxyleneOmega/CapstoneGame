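; TestMango is a test consumable item Blueprint in the inventory system.
; Its Consumption event increments the consuming character's Health and prints the new value.
; LookAt checks the item's data table row from its ItemDataComponent, then creates a look-at pickup widget for that ItemID, adds it to the viewport and returns it.
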(event EventConsumption
  (params (PlayerCharacter :type BP%20CG%20Char%20Object%20Reference))
  (bind _result (Math|Integer|IncrementInt (Variables|/Game/Capstone/BP_CG_Char.BP_CG_Char_C|GetHealth PlayerCharacter))
    (:%20%20
      (Development|PrintString (Utilities|String|ToString(Integer) _result)))))

(fn ConstructionScript)

(fn Lookat
  (bind _itemdatacomponent (Variables|Default|GetItemDataComponent))
  (bind _itemid (Variables|/Game/Capstone/Inventory/Blueprints/ItemDataComponent.ItemDataComponent_C|GetItemID _itemdatacomponent))
  (bind _returnvalue (Utilities|GetDataTableRow (.datatable _itemid) (.rowname _itemid))
    (:then
      (bind _returnvalue_2 (UserInterface|CreateWidget "/Game/Capstone/Inventory/Widgets/W_LookAtPickableItem.W_LookAtPickableItem_C" 0 (.rowname _itemid)))
      (UserInterface|Viewport|AddtoViewport _returnvalue_2 0)
      (return _returnvalue_2))))