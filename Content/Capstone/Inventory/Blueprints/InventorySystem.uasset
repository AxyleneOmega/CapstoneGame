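; Inventory component for the player character that stores items in fixed-size slots and handles look-at interaction.
; Each tick a camera sphere trace updates the looked-at actor and its widget; F messages that actor's ItemDataComponent to interact.
; AddToInventory fills matching stacks up to data-table limits, then empty slots, one unit at a time.
; Removal is an empty stub, AddToInventory's Success returns the failure flag, and key 1 prints contents.
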(event EventBeginPlay
  (Utilities|Array|Resize (Variables|Default|GetContent) (Variables|Default|GetInventorySize)))

(event EventTick
  (params (DeltaSeconds :type Float%20%28single-precision%29))
  (CallFunction|InteractionTrace))

(event Input|KeyboardEvents|1
  (params (Key :type Key%20Structure :default "None"))
  (:Pressed
    (CallFunction|DebugPrintContents)))

(event Input|KeyboardEvents|F
  (params (Key :type Key%20Structure :default "None"))
  (:Pressed
    (bind _lookatactor (Variables|Default|GetLookAtActor)
      (:then
        (Class|IInteract|Interactwith(Message) (Actor|GetComponentbyClass _lookatactor "/Game/Capstone/Inventory/Blueprints/ItemDataComponent.ItemDataComponent_C") (.AsBP%20CG%20Char (Utilities|Casting|CastToBP_CG_Char (Components|GetOwner)))))
      (:else))))

(fn AddtoInventory
  (params (ItemID :type Name) (Quantity :type Integer))
  (LocalVariables|SetLocal_QuantityRemaining Quantity)
  (while (and (> (LocalVariables|GetLocal_QuantityRemaining) 0) (not (LocalVariables|GetLocal_HasFailed)))
    (bind (_index _foundslot) (CallFunction|FindSlot ItemID))
    (if _foundslot
      (CallFunction|AddtoStack _index 1)
      (Math|Integer|DecrementInt (LocalVariables|GetLocal_QuantityRemaining))
      (elif (.IsEmptySlot (CallFunction|AnyEmptySlotAvailable))
        (bind _success (CallFunction|CreateNewStack ItemID 1))
        (if _success
          (Math|Integer|DecrementInt (LocalVariables|GetLocal_QuantityRemaining))
          (else
            (LocalVariables|SetLocal_HasFailed true)))
        (else
          (LocalVariables|SetLocal_HasFailed true)))))
  (return (LocalVariables|GetLocal_HasFailed) (LocalVariables|GetLocal_QuantityRemaining)))

(fn RemovefromInventory)

(fn InteractionTrace
  (bind _returnvalue (Game|GetPlayerCameraManager 0))
  (bind _returnvalue_2 (Transformation|GetActorLocation _returnvalue))
  (bind (_outhit _returnvalue_3) (Collision|SphereTraceByChannel _returnvalue_2 (+ (* (Transformation|GetActorForwardVector _returnvalue) (Variables|Default|GetInteractionRange)) _returnvalue_2) 15.0 "TraceTypeQuery3" false (Utilities|Array|MakeArray (Components|GetOwner)) "None"))
  (if _returnvalue_3
    (if (!= (.HitActor (Collision|BreakHitResult _outhit)) (Variables|Default|GetLookAtActor))
      (bind _output_get (Variables|Default|SetLookAtActor (.HitActor (Collision|BreakHitResult _outhit))))
      (bind _lookatwidget (Class|IInteract|Lookat(Message) _output_get))
      (Variables|Default|SetLookAtWidget _lookatwidget))
    (else
      (Variables|Default|SetLookAtActor 0)
      (bind _lookatwidget_2 (Variables|Default|GetLookAtWidget)
        (:then
          (Widget|RemovefromParent _lookatwidget_2))
        (:else)))))

(fn FindSlot
  (params (ItemID :type Name))
  (for (_array_element _array_index) (Variables|Default|GetContent)
    (if (== (.ItemID (Utilities|Struct|BreakFSlotStructure _array_element)) ItemID)
      (if (< (.Quantity (Utilities|Struct|BreakFSlotStructure _array_element)) (CallFunction|GetMaxStackSize ItemID))
        (return _array_index true))))
  (return -1 false))

(fn GetMaxStackSize
  (params (ItemID :type Name))
  (bind _returnvalue (Utilities|GetDataTableRow "/Game/Capstone/Inventory/ItemData.ItemData" ItemID)
    (:then
      (return (Utilities|Struct|BreakFItemStructure _returnvalue)))
    (:RowNotFound
      (return -1))))

(fn AddtoStack
  (params (Index :type Integer) (Quantity :type Integer))
  (bind _content (Variables|Default|GetContent))
  (bind _output (Utilities|Array|Get(acopy) _content Index))
  (Utilities|Array|SetArrayElem (Variables|Default|GetContent) Index (Utilities|Struct|MakeFSlotStructure (.itemid _output) (+ (.quantity _output) Quantity))))

(fn AnyEmptySlotAvailable
  (for (_array_element _array_index) (Variables|Default|GetContent)
    (if (== (.Quantity (Utilities|Struct|BreakFSlotStructure _array_element)) 0)
      (return true _array_index)))
  (return false -1))

(fn CreateNewStack
  (params (ItemID :type Name) (Quantity :type Integer))
  (bind (_isemptyslot _emptyindex) (CallFunction|AnyEmptySlotAvailable))
  (if _isemptyslot
    (Utilities|Array|SetArrayElem (Variables|Default|GetContent) _emptyindex (Utilities|Struct|MakeFSlotStructure ItemID Quantity))
    (return true)
    (else
      (return false))))

(fn DebugPrintContents
  (for (_array_element _array_index) (Variables|Default|GetContent)
    (Development|PrintString (Utilities|String|Append (Utilities|String|ToString(Integer) _array_index) ":" (Utilities|String|ToString(Name) (.ItemID (Utilities|Struct|BreakFSlotStructure _array_element))) ":" (Utilities|String|ToString(Integer) (.Quantity (Utilities|Struct|BreakFSlotStructure _array_element)))))))