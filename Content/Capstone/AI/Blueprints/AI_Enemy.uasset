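; AI controller for enemies that starts the BT_Enemy behavior tree on BeginPlay and feeds it what the enemy perceives.
; Perception updates go to hearing and sight handlers, each filtering by sense class and writing to the Blackboard.
; Successful hearing stores LastHeardLocation.
; Sight reacts only to the player character, setting TargetActor while seen, then clearing it and storing LastSeenLocation when sight is lost.
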(event OnTargetPerceptionUpdated(AIPerception)
  (params (Actor :type Actor%20Object%20Reference) (Stimulus :type AI%20Stimulus%20Structure))
  (CallFunction|HearSensing Stimulus)
  (CallFunction|SightSensing Stimulus Actor))

(event EventBeginPlay
  (AI|RunBehaviorTree "/Game/Capstone/AI/BehaviourTrees/BT_Enemy.BT_Enemy"))

(event EventTick
  (params (DeltaSeconds :type Float%20%28single-precision%29)))

(fn ConstructionScript)

(fn HearSensing
  (params (Stimulus :type AI%20Stimulus%20Structure))
  (bind (_age _expirationage _strength _stimuluslocation _receiverlocation _tag _bsuccessfullysensed) (Utilities|Struct|BreakAIStimulus Stimulus))
  (bind _returnvalue (Class|AIPerceptionSystem|GetSenseClassforStimulus Stimulus))
  (if (== _returnvalue "/Script/AIModule.AISense_Hearing")
    (if _bsuccessfullysensed
      (AI|Components|Blackboard|SetValueasVector (AI|GetBlackboard 0) (Utilities|Name|MakeLiteralName "LastHeardLocation") _stimuluslocation))))

(fn SightSensing
  (params (Stimulus :type AI%20Stimulus%20Structure) (Actor :type Actor%20Object%20Reference))
  (bind (_age _expirationage _strength _stimuluslocation _receiverlocation _tag _bsuccessfullysensed) (Utilities|Struct|BreakAIStimulus Stimulus))
  (bind _returnvalue (Class|AIPerceptionSystem|GetSenseClassforStimulus Stimulus))
  (if (== _returnvalue "/Script/AIModule.AISense_Sight")
    (if (== Actor (Game|GetPlayerCharacter 0))
      (AI|Components|Blackboard|SetValueasObject (AI|GetBlackboard 0) (Utilities|Name|MakeLiteralName "TargetActor") (Utilities|SelectObject (Game|GetPlayerCharacter 0) 0 _bsuccessfullysensed))
      (if (not _bsuccessfullysensed)
        (AI|Components|Blackboard|SetValueasVector (AI|GetBlackboard 0) (Utilities|Name|MakeLiteralName "LastSeenLocation") _stimuluslocation)))))