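; BP_NPC is an interactable NPC that shows its interaction state on a widget.
; Every Tick it compares the player character's distance with its interaction range, then refreshes the widget text to show interactable, already interacted or blank.
; It stores its spawn location as home on BeginPlay; neither that nor the interacted flag's setting is used or handled here.
; The construction script tints the Manny mesh cyan through dynamic material instances.
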(event Custom|UpdateText
  ;[1 1 1] Text Update for Interactable/Interacted NPCs
  (bind _asbp_npcinteraction (Utilities|Casting|CastToBP_NPCInteraction (UserInterface|GetUserWidgetObject (Variables|Default|GetWidget))))
  (if (Variables|Default|GetIsInteracted)
    (Variables|/Script/UMG.TextBlock|SetText (Variables|/Game/Capstone/Blueprints/Widgets/BP_NPCInteraction.BP_NPCInteraction_C|GetInteraction _asbp_npcinteraction) "Interacted.")
    (elif (Variables|Default|GetIsInRange)
      (Variables|/Script/UMG.TextBlock|SetText (Variables|/Game/Capstone/Blueprints/Widgets/BP_NPCInteraction.BP_NPCInteraction_C|GetInteraction _asbp_npcinteraction) "Interactable")
      (else
        (Variables|/Script/UMG.TextBlock|SetText (Variables|/Game/Capstone/Blueprints/Widgets/BP_NPCInteraction.BP_NPCInteraction_C|GetInteraction _asbp_npcinteraction) "")))))

(event EventBeginPlay
  (Variables|Default|SetHomeLocation (Transformation|GetActorLocation)))

(event Collision|EventActorBeginOverlap
  (params (OtherActor :type Actor%20Object%20Reference)))

(event EventTick
  (params (DeltaSeconds :type Float%20%28single-precision%29))
  ;[1 1 1] Checking if NPC within range of interaction
  (if (<= (Math|Vector|Distance(Vector) (Transformation|GetActorLocation (Game|GetPlayerCharacter 0)) (Transformation|GetActorLocation)) (Variables|Default|GetRangeOfInteraction))
    (Variables|Default|SetIsInRange true)
    (else
      (Variables|Default|SetIsInRange false)))
  (CallFunction|UpdateText))

(fn ConstructionScript
  (bind _mesh (Variables|Character|GetMesh))
  (bind _returnvalue (Rendering|Material|CreateDynamicMaterialInstance _mesh 0 "/Game/Characters/Mannequins/Materials/Instances/Manny/MI_Manny_02.MI_Manny_02" "None" :!class /Script/Engine.PrimitiveComponent))
  (bind _returnvalue_2 (Rendering|Material|CreateDynamicMaterialInstance _mesh 1 "/Game/Characters/Mannequins/Materials/Instances/Manny/MI_Manny_01.MI_Manny_01" "None" :!class /Script/Engine.PrimitiveComponent))
  (Rendering|Material|SetVectorParameterValue _returnvalue "Tint" "(R=0.000000,G=1.000000,B=1.500000,A=1.000000)" :!class /Script/Engine.MaterialInstanceDynamic))